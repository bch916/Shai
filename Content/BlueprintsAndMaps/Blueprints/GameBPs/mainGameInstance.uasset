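; Game instance for an RPG that carries player and enemy state between the overworld and battles.
; Overworld enemies spawn from level and enemy data tables, or from tracked active spawns in dev mode, at random offsets around an origin.
; It caches the battle enemy's stats, relays its damage to battleGameMode, then awards exp and formula-based level-ups unless the player fled.
; A constructed PlayerObjectBP holds player stats, set up on new game or load and saved on quit.
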(event Custom|QuitAndSaveGame
  ;[1 1 1] Quit and Save game from Overworld UI. Setting variables to Player Save Struct
  (Default|UpdatePlayerStatsStructurefromREF (Variables|Default|GetMainGameInstancePlayerObjectBP))
  (bind _returnvalue (SaveGame|CreateSaveGameObject "/Game/BlueprintsAndMaps/Blueprints/GameBPs/PlayerSaveGameObject.PlayerSaveGameObject_C"))
  (bind _output_get (Variables|Default|SetcurrentPlayerSaveGameObject _returnvalue))
  (Variables|/Game/BlueprintsAndMaps/Blueprints/GameBPs/PlayerSaveGameObject.PlayerSaveGameObject_C|SetREFPlayerStatsStructure _output_get (Variables|/Game/BlueprintsAndMaps/Blueprints/PlayerBPs/playerObjectBP.playerObjectBP_C|GetplayerStatsStructure (Variables|Default|GetMainGameInstancePlayerObjectBP)))
  (bind _returnedplayersaveslot (Default|ReturnPlayerSaveSlot (Variables|Default|GetMainGameInstancePlayerObjectBP)))
  (SaveGame|SaveGametoSlot (Variables|Default|GetcurrentPlayerSaveGameObject) _returnedplayersaveslot)
  (Game|QuitGame (Game|GetPlayerController 0) "Quit" false))

(event Custom|updatePlayerOnLoad
  (params (loadedPlayerSaveObject :type Player%20Stats%20Structure%20Structure))
  (bind (_playercurrenthealth _playermaxhealth _playerexp _playerexptonextlevel _playerlevel _playerbasepower _profilename _playersaveslot _previousplayerexptonextlevel _currentlevelname _playerallweapons _playerallskills _playerequippedskills) (Utilities|Struct|BreakPlayerStatsStructure loadedPlayerSaveObject))
  (bind _maingameinstanceplayerobjectbp (Variables|Default|GetMainGameInstancePlayerObjectBP))
  ;[1 1 1] Updates Player on Load of Game from save Game Object. Updates our current Structure of the Player
  (CallFunction|ConstructPlayerObject)
  (Default|UpdatePlayerStatsStructurefromSaveGameObject (Variables|Default|GetMainGameInstancePlayerObjectBP) loadedPlayerSaveObject)
  (Default|LoadInventory _maingameinstanceplayerobjectbp _playerallweapons)
  (Default|AddSkilltoAllSkillsbySkillData _maingameinstanceplayerobjectbp _playerallskills)
  (Default|AddSkilltoEquippedbyData (Variables|Default|GetMainGameInstancePlayerObjectBP) _playerequippedskills)
  (Default|CalcTotalPower (Variables|Default|GetMainGameInstancePlayerObjectBP)))

(event Custom|loadEnemiesByLevel
  (params (levelName :type Name))
  ;[1 1 1] Prototype Enemy Spawn by level name event. We will call this on New Game/Load Game and map change.
  (CallFunction|SetLoadedEnemiesArraybyLevel levelName)
  (CallFunction|SpawnLoadedEnemies))

(event Custom|playerEnteredLevel
  ;[1 1 1] Prototype Enemy Spawn by level name event. We will call this on New Game/Load Game and map change.
  (if (Variables|Default|GetisDevMode)
    (CallFunction|SetLoadedEnemiesbyActiveMobSpawns (Variables|Default|GetactiveMobSpawns))
    (CallFunction|SpawnLoadedEnemies)
    (else
      (bind _returnvalue (Game|GetCurrentLevelName true))
      (bind _output_get (Variables|/Game/BlueprintsAndMaps/Blueprints/PlayerBPs/playerObjectBP.playerObjectBP_C|SetREFCurrentLevelName (Variables|Default|GetMainGameInstancePlayerObjectBP) (Utilities|String|StringToName _returnvalue)))
      (CallFunction|LoadEnemiesbyLevel _output_get))))

(event Custom|calculateDamageCurrentBattleEnemyBySkillIndex
  (params (skillIndex :type Integer))
  (bind _currentbattleenemyoverworlddata (Variables|Default|GetcurrentBattleEnemyOverworldData))
  ;[1 1 1] Updated Enemy Damage System for Battle
  (Default|UpdateEnemyPower _currentbattleenemyoverworlddata)
  (bind _damagebyskill (Default|CalcDamagebySkillIndex _currentbattleenemyoverworlddata skillIndex))
  (bind _asbattle_game_mode (Utilities|Casting|CastTobattleGameMode (Game|GetGameMode)))
  (Default|ApplyDamage _asbattle_game_mode false _damagebyskill))

(event Custom|loadEnemyByName
  (params (enemyName :type Name))
  (bind (_activemobspawndata _addedenemypawn) (CallFunction|SpawnSingleEnemyatDefaultLocation enemyName))
  (bind _returnvalue (Utilities|Array|Add (Variables|Default|GetactiveMobSpawns) _activemobspawndata))
  (Variables|/Game/BlueprintsAndMaps/Blueprints/EnemyBPs/Demo_BPs/overWorldEnemyPawnBP.overWorldEnemyPawnBP_C|SetcurrentEnemyIndex _addedenemypawn _returnvalue))

(event Custom|changeMobSpawnCount
  (params (activeMobNum :type Integer) (defeateEnemyData :type Enemy%20Data%20Structure%20Structure) (enemyIndex :type Integer))
  ;[1 1 1] Game Instance wants to keep track of how many Mobs should currently be spawning on this tile.
  (Utilities|Array|RemoveIndex (Variables|Default|GetactiveMobSpawns) enemyIndex)
  (Variables|Default|SetcurrentMobCount (- (Variables|Default|GetcurrentMobCount) activeMobNum))
  (bind _asbattle_game_mode (Utilities|Casting|CastTobattleGameMode (Game|GetGameMode)))
  (Default|DisplayEndBattleScreen _asbattle_game_mode))

(event Custom|setBattleEnemyType
  (params (overWorldPawnEnemyREF :type Over%20World%20Enemy%20Pawn%20BP%20Object%20Reference))
  ;[1 1 1] Game Instance can Set the Enemy Battle type so that the Battle Game Mode will know what Enemy is battling. Storing some reward information ehre like Exp for now since it is a great time to get this data off the enemy while the referenc is valid.
  (Variables|Default|SetREF_BattleEnemyType (Utilities|GetClass overWorldPawnEnemyREF))
  (bind _output_get (Variables|Default|SetcurrentBattleEnemyOverworldData overWorldPawnEnemyREF))
  (Variables|Default|SetcurrentBattleEnemyData (Variables|/Game/BlueprintsAndMaps/Blueprints/EnemyBPs/enemyObject_BP.enemyObject_BP_C|GetenemyDataStructure (Variables|/Game/BlueprintsAndMaps/Blueprints/EnemyBPs/Demo_BPs/overWorldEnemyPawnBP.overWorldEnemyPawnBP_C|GetenemyObject _output_get)))
  (Variables|Default|SetcurrentEnemyHealth (Variables|/Game/BlueprintsAndMaps/Blueprints/EnemyBPs/Demo_BPs/overWorldEnemyPawnBP.overWorldEnemyPawnBP_C|GetREFCurrentHealth (Variables|Default|GetcurrentBattleEnemyOverworldData)))
  (Variables|Default|SetcurrentEnemyMaxHealth (Variables|/Game/BlueprintsAndMaps/Blueprints/EnemyBPs/Demo_BPs/overWorldEnemyPawnBP.overWorldEnemyPawnBP_C|GetREFMaxHealth (Variables|Default|GetcurrentBattleEnemyOverworldData)))
  (Variables|Default|SetcurrentEnemyExpOnDefeat (Variables|/Game/BlueprintsAndMaps/Blueprints/EnemyBPs/Demo_BPs/overWorldEnemyPawnBP.overWorldEnemyPawnBP_C|GetexpGivenOnDefeat (Variables|Default|GetcurrentBattleEnemyOverworldData)))
  (Default|UpdateEnemyStatsfromREF (Variables|Default|GetcurrentBattleEnemyOverworldData)))

(event Custom|UpdatePlayerAfterBattle
  (bind _maingameinstanceplayerobjectbp (Variables|Default|GetMainGameInstancePlayerObjectBP))
  (bind _currentenemyexpondefeat (Variables|Default|GetcurrentEnemyExpOnDefeat))
  ;[1 1 1] Current Update we call at end of Battle. Checks if we flee'd and if not gives us our loot and or levels us up.
  (if (Variables|Default|GetplayerFlee?)
    (Variables|Default|SetplayerFlee? false)
    (else
      (Variables|Default|SetTempPlayerCurrentExp (+ (Math|Random|RandomIntegerinRange (Utilities|Array|Get(acopy) _currentenemyexpondefeat) (Utilities|Array|Get(acopy) _currentenemyexpondefeat 1)) (Variables|/Game/BlueprintsAndMaps/Blueprints/PlayerBPs/playerObjectBP.playerObjectBP_C|GetREFPlayerCurrentExp _maingameinstanceplayerobjectbp)))
      (if (>= (Variables|Default|GetTempPlayerCurrentExp) (Variables|/Game/BlueprintsAndMaps/Blueprints/PlayerBPs/playerObjectBP.playerObjectBP_C|GetREFPlayerExpToNextLevel _maingameinstanceplayerobjectbp))
        (CallFunction|LevelUpPlayer)
        (else
          (Variables|/Game/BlueprintsAndMaps/Blueprints/PlayerBPs/playerObjectBP.playerObjectBP_C|SetREFPlayerCurrentExp (Variables|Default|GetMainGameInstancePlayerObjectBP) (Variables|Default|GetTempPlayerCurrentExp))))
      (Default|UpdatePlayerStatsStructurefromREF (Variables|Default|GetMainGameInstancePlayerObjectBP)))))

(event Custom|endBattle
  ;[1 1 1] Game Instance is Ending Battle and Opening Overworld Map. Opening the next level should definately be on Battle Game Mode and may be redundant here. Prototype Level Up system for Save Game Prototype here currently.
  (CallFunction|UpdatePlayerAfterBattle)
  (Game|OpenLevel(byName) "OverWorldMap"))

(event Custom|levelUpPlayer
  ;[1 1 1] Calls two fn.'s that add to player Max HP and set the Exp to Next Level. Weird shit in the fns. check google sheets.
  (Variables|Default|SetTempPreviousPlayerExpToNextLevel (Variables|/Game/BlueprintsAndMaps/Blueprints/PlayerBPs/playerObjectBP.playerObjectBP_C|GetREFPlayerExpToNextLevel (Variables|Default|GetMainGameInstancePlayerObjectBP)))
  (bind _output_get (Variables|Default|SetTempPlayerLevel (Variables|/Game/BlueprintsAndMaps/Blueprints/PlayerBPs/playerObjectBP.playerObjectBP_C|GetREFPlayerLevel (Variables|Default|GetMainGameInstancePlayerObjectBP))))
  (Math|Integer|IncrementInt _output_get
    (:%20%20
      (Variables|Default|SetTempPlayerMaxHealth (Math|Conversions|ToFloat(Integer) (Variables|/Game/BlueprintsAndMaps/Blueprints/PlayerBPs/playerObjectBP.playerObjectBP_C|GetREFPlayerMaxHealth (Variables|Default|GetMainGameInstancePlayerObjectBP))))
      (bind _retbonushealth (CallFunction|CalcBonusHPonLevel (Variables|Default|GetTempPlayerLevel)))
      (Variables|Default|SetTempPlayerMaxHealth (+ (Math|Conversions|ToFloat(Integer) _retbonushealth) (Variables|Default|GetTempPlayerMaxHealth)))
      (Variables|/Game/BlueprintsAndMaps/Blueprints/PlayerBPs/playerObjectBP.playerObjectBP_C|SetREFPlayerPreviousExpToNextLevel (Variables|Default|GetMainGameInstancePlayerObjectBP) (Variables|Default|GetTempPlayerExpToNextLevel))
      (bind _exptonextlevel (CallFunction|CalcExptoNextLevel (Variables|Default|GetTempPlayerLevel)))
      (Variables|Default|SetTempPlayerExpToNextLevel _exptonextlevel)
      (Variables|/Game/BlueprintsAndMaps/Blueprints/PlayerBPs/playerObjectBP.playerObjectBP_C|SetREFPlayerCurrentExp (Variables|Default|GetMainGameInstancePlayerObjectBP) (Variables|Default|GetTempPlayerCurrentExp))
      (Variables|/Game/BlueprintsAndMaps/Blueprints/PlayerBPs/playerObjectBP.playerObjectBP_C|SetREFPlayerExpToNextLevel (Variables|Default|GetMainGameInstancePlayerObjectBP) (Variables|Default|GetTempPlayerExpToNextLevel))
      (Variables|/Game/BlueprintsAndMaps/Blueprints/PlayerBPs/playerObjectBP.playerObjectBP_C|SetREFPlayerLevel (Variables|Default|GetMainGameInstancePlayerObjectBP) (Variables|Default|GetTempPlayerLevel))
      (Variables|/Game/BlueprintsAndMaps/Blueprints/PlayerBPs/playerObjectBP.playerObjectBP_C|SetREFPlayerMaxHealth (Variables|Default|GetMainGameInstancePlayerObjectBP) (Math|Float|Truncate (Variables|Default|GetTempPlayerMaxHealth))))))

(event Custom|openInventoryUI
  ;[1 1 1] Prototype For Inventory UI..integrates Instantiating an Inventory Object on the player at the game intances call, ref the game isntance player object on the inventory UI to get all weapons and display them.
  (bind _returnvalue (UserInterface|CreateWidget "/Game/BlueprintsAndMaps/Blueprints/UI_BPs/PlayerWeaponSkillsUI.PlayerWeaponSkillsUI_C"))
  (UserInterface|Viewport|AddtoViewport _returnvalue 0))

(event Custom|updatePlayerNewGame
  (bind _maingameinstanceplayerobjectbp (Variables|Default|GetMainGameInstancePlayerObjectBP))
  (bind _starterskills (Variables|/Game/BlueprintsAndMaps/Blueprints/PlayerBPs/playerObjectBP.playerObjectBP_C|GetStarterSkills _maingameinstanceplayerobjectbp))
  ;[1 1 1] Player Initialization code goes here for now.
  (CallFunction|ConstructPlayerObject)
  (Default|UpdateREFVariablesfromPlayerStatsStructure (Variables|Default|GetMainGameInstancePlayerObjectBP))
  ;;[1 1 1] Gives our player testable weapons and skills on new game.
  (Default|PlayerAquiresWeapon (Variables|Default|GetMainGameInstancePlayerObjectBP) "WoodStick")
  (Default|PlayerAquiresSkill _maingameinstanceplayerobjectbp _starterskills)
  (Default|AddSkilltoEquippedbyName (Variables|Default|GetMainGameInstancePlayerObjectBP) _starterskills)
  (Variables|/Game/BlueprintsAndMaps/Blueprints/PlayerBPs/playerObjectBP.playerObjectBP_C|SetREFProfileName (Variables|Default|GetMainGameInstancePlayerObjectBP) (Variables|Default|GetProfileName))
  (Variables|/Game/BlueprintsAndMaps/Blueprints/PlayerBPs/playerObjectBP.playerObjectBP_C|SetREFPlayerSaveSlot (Variables|Default|GetMainGameInstancePlayerObjectBP) (Variables|Default|GetPlayerSaveSlot))
  (Default|UpdatePlayerStatsStructurefromREF (Variables|Default|GetMainGameInstancePlayerObjectBP)))

(event Custom|constructPlayerObject
  ;[1 1 1] Creates an Instance of PlayerObject for use on Load or New Game
  (bind _returnvalue (Game|ConstructObjectfromClass "/Game/BlueprintsAndMaps/Blueprints/PlayerBPs/playerObjectBP.playerObjectBP_C" self))
  (Variables|Default|SetMainGameInstancePlayerObjectBP _returnvalue))

(fn CalcBonusHPonLevel
  (params (playerLevel :type Integer))
  (LocalVariables|SetplayerLevelREF playerLevel)
  (bind _output_get (LocalVariables|SettotalBonusHP (Math|Float|Truncate (* (* (LocalVariables|GetplayerLevelREF) (LocalVariables|GetHealthPiValue)) (* (LocalVariables|GetplayerLevelREF) (LocalVariables|GetHealthGoldenRatio))))))
  (return _output_get))

(fn CalcExptoNextLevel
  (params (PlayerLevel :type Integer))
  ;[1 1 1] Check google sheets player scaling for explanation of this weird shit.
  (LocalVariables|SetplayerLevelREF PlayerLevel)
  (LocalVariables|SetpumpUpValue (* (LocalVariables|GetplayerLevelREF) (LocalVariables|GetbaseValue)))
  (LocalVariables|SetAddedVariationValue (* (Math|Float|Power (Math|Conversions|ToFloat(Integer) (LocalVariables|GetplayerLevelREF)) 1.6) 1e+02))
  (LocalVariables|SetLevelMultiplierValue (Math|Float|Power 1.6 (Math|Conversions|ToFloat(Integer) (LocalVariables|GetplayerLevelREF))))
  (return (+ (Math|Float|Floor (LocalVariables|GetAddedVariationValue)) (Math|Float|Truncate (* (LocalVariables|GetLevelMultiplierValue) (LocalVariables|GetpumpUpValue))))))

(fn SetLoadedEnemiesArraybyLevel
  (params (levelByName :type Name))
  (bind _returnvalue (Utilities|GetDataTableRow "/Game/BlueprintsAndMaps/Blueprints/GameBPs/LevelBPs/LevelDataTable.LevelDataTable" levelByName)
    (:then
      (for _array_element (.enemiesToSpawnByName (Utilities|Struct|BreakLevelDataStructure _returnvalue))
        (Utilities|Array|Add (Variables|Default|GetLoadedEnemiesByName) _array_element)
        (return)))))

(fn SpawnLoadedEnemies
  (bind _overworldenemyorigin (Variables|Default|GetoverworldEnemyOrigin))
  (for (_array_element _array_index) (Variables|Default|GetLoadedEnemiesByName)
    (bind _returnvalue (Utilities|GetDataTableRow "/Game/BlueprintsAndMaps/Blueprints/EnemyBPs/EnemyDataTable.EnemyDataTable" _array_element)
      (:then
        (bind _returnvalue_2 (Game|SpawnActorfromClass (.enemyClass (Utilities|Struct|BreakEnemyDataStructure _returnvalue)) (Math|Transform|MakeTransform (Math|Vector|MakeVector (+ (.x _overworldenemyorigin) (Math|Random|RandomFloatinRange -5e+02 5e+02)) (+ (.y _overworldenemyorigin) (Math|Random|RandomFloatinRange -5e+02 5e+02)) (.z _overworldenemyorigin)) "0,180.000000, 0") "AdjustIfPossibleButAlwaysSpawn" 0 _array_index 0))
        (bind _returnvalue_3 (Game|ConstructObjectfromClass "/Game/BlueprintsAndMaps/Blueprints/EnemyBPs/enemyObject_BP.enemyObject_BP_C" _returnvalue_2))
        (bind _output_get (Variables|/Game/BlueprintsAndMaps/Blueprints/EnemyBPs/Demo_BPs/overWorldEnemyPawnBP.overWorldEnemyPawnBP_C|SetenemyObject _returnvalue_2 _returnvalue_3))
        (Variables|/Game/BlueprintsAndMaps/Blueprints/EnemyBPs/enemyObject_BP.enemyObject_BP_C|SetenemyDataStructure _output_get _returnvalue)
        (Default|SetEnemytoOverWorldState _returnvalue_2)
        (Default|UpdateEnemyREFfromStats _returnvalue_2))))
  (return))

(fn SpawnSingleEnemyatDefaultLocation
  (params (enemyName :type Name))
  (bind _overworldenemyorigin (Variables|Default|GetoverworldEnemyOrigin))
  (bind _returnvalue (Utilities|GetDataTableRow "/Game/BlueprintsAndMaps/Blueprints/EnemyBPs/EnemyDataTable.EnemyDataTable" enemyName)
    (:then
      (bind _returnvalue_2 (Game|SpawnActorfromClass (.enemyClass (Utilities|Struct|BreakEnemyDataStructure _returnvalue)) (Math|Transform|MakeTransform (Math|Vector|MakeVector (+ (.x _overworldenemyorigin) (Math|Random|RandomFloatinRange -5e+02 5e+02)) (+ (.y _overworldenemyorigin) (Math|Random|RandomFloatinRange -5e+02 5e+02)) (.z _overworldenemyorigin)) "0,180.000000, 0") "AdjustIfPossibleButAlwaysSpawn" 0 0 0))
      (bind _output_get (LocalVariables|SetRETenemiesToAdd _returnvalue_2))
      (bind _returnvalue_3 (Game|ConstructObjectfromClass "/Game/BlueprintsAndMaps/Blueprints/EnemyBPs/enemyObject_BP.enemyObject_BP_C" _output_get))
      (bind _output_get_2 (Variables|/Game/BlueprintsAndMaps/Blueprints/EnemyBPs/Demo_BPs/overWorldEnemyPawnBP.overWorldEnemyPawnBP_C|SetenemyObject (LocalVariables|GetRETenemiesToAdd) _returnvalue_3))
      (Variables|/Game/BlueprintsAndMaps/Blueprints/EnemyBPs/enemyObject_BP.enemyObject_BP_C|SetenemyDataStructure _output_get_2 _returnvalue)
      (Default|SetEnemytoOverWorldState (LocalVariables|GetRETenemiesToAdd))
      (Default|UpdateEnemyREFfromStats (LocalVariables|GetRETenemiesToAdd))
      (return (Variables|/Game/BlueprintsAndMaps/Blueprints/EnemyBPs/enemyObject_BP.enemyObject_BP_C|GetenemyDataStructure (Variables|/Game/BlueprintsAndMaps/Blueprints/EnemyBPs/Demo_BPs/overWorldEnemyPawnBP.overWorldEnemyPawnBP_C|GetenemyObject (LocalVariables|GetRETenemiesToAdd))) (LocalVariables|GetRETenemiesToAdd)))))

(fn SetLoadedEnemiesbyActiveMobSpawns
  (params (activeMobSpawns :type Array%20of%20Enemy%20Data%20Structure%20Structures))
  (Utilities|Array|Clear (Variables|Default|GetLoadedEnemiesByName))
  (for _array_element activeMobSpawns
    (Utilities|Array|Add (Variables|Default|GetLoadedEnemiesByName) (Utilities|String|StringToName (.enemyName (Utilities|Struct|BreakEnemyDataStructure _array_element)))))
  (return))