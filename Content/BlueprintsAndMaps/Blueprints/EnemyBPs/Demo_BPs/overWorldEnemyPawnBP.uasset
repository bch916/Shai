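; Slime enemy pawn serving both the overworld and turn-based battle, swapping anim Blueprints per state and halting non-engaging players who overlap it in the overworld.
; Stats are mirrored between its EnemyObject data struct and REF variables, with skill damage rolled from base power.
; Damage updates the active game mode's UI and GameInstance, destroying the pawn on defeat.
; Its delayed turn sets attack or shoot flags, then notifies the battle game mode.
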(event Custom|enemyTargeted
  ;[1 1 1] Interaction from Player Controller can call this event to set Enemy into Reacting State
  (Variables|Default|SetisReacting true))

(event Custom|takeDamage
  (params (damageNumber :type Integer))
  (bind _returnvalue (Game|GetGameMode))
  ;[1 1 1] Enemy Takes Damage.  Subtract incoming damage from health and pass the damage number to the Game Modes Current UI to display dmg.
  (Variables|Default|SetREFCurrentHealth (- (Variables|Default|GetREFCurrentHealth) (Math|Conversions|ToFloat(Integer) damageNumber)))
  (bind _asmain_game_mode (Utilities|Casting|CastTomainGameMode _returnvalue)
    (:then
      (Variables|/Game/BlueprintsAndMaps/Blueprints/UI_BPs/OverworldUI.OverworldUI_C|SetenemyDamagedNumber (Variables|/Game/BlueprintsAndMaps/Blueprints/GameBPs/mainGameMode.mainGameMode_C|GetcurrentOverworldUI _asmain_game_mode) damageNumber)
      (Default|EnemyTakesDamage (Variables|/Game/BlueprintsAndMaps/Blueprints/GameBPs/mainGameMode.mainGameMode_C|GetcurrentOverworldUI _asmain_game_mode) damageNumber))
    (:CastFailed
      (bind _asbattle_game_mode (Utilities|Casting|CastTobattleGameMode _returnvalue))
      (bind _output_get (Variables|/Game/BlueprintsAndMaps/Blueprints/UI_BPs/BattleUI.BattleUI_C|SetenemyDamagedNumber (Variables|/Game/BlueprintsAndMaps/Blueprints/GameBPs/battleGameMode.battleGameMode_C|GetcurrentBattleUIInstance _asbattle_game_mode) damageNumber))
      (Default|EnemyTakesDamage (Variables|/Game/BlueprintsAndMaps/Blueprints/GameBPs/battleGameMode.battleGameMode_C|GetcurrentBattleUIInstance _asbattle_game_mode) _output_get)))
  ;[1 1 1] Check if Damage is defating the Enemy and if so set Flag fo Defeated and call Change Mob Spawn Count on Game Instance. Delay 1 second and DEstroy the Enemy Pawn.
  (if (<= (Variables|Default|GetREFCurrentHealth) 0.0)
    (Variables|Default|SetisDefeated true)
    (Default|ChangeMobSpawnCount (.AsMain%20Game%20Instance (Utilities|Casting|CastTomainGameInstance (Game|GetGameInstance))) 1)
    (Utilities|FlowControl|Delay 1.0)
    (Actor|DestroyActor)
    (else
      (Variables|/Game/BlueprintsAndMaps/Blueprints/GameBPs/mainGameInstance.mainGameInstance_C|SetcurrentEnemyHealth (.AsMain%20Game%20Instance (Utilities|Casting|CastTomainGameInstance (Game|GetGameInstance))) (Variables|Default|GetREFCurrentHealth))
      (CallFunction|UpdateEnemyStatsfromREF))))

(event Custom|updateEnemyPower
  (CallFunction|SetEnemyPower))

(event Custom|setEnemyToBattleState
  (Class|SkeletalMeshComponent|SetAnimClass (Variables|Default|GetenemyMesh) "/Game/myModels/EnemyAnims/slimeBatlleAnimBP.slimeBatlleAnimBP_C")
  (Components|Activation|Deactivate (Variables|Default|GetOverLapSphere))
  (Transformation|SetActorRotation "0,-90.000000, 0")
  (CallFunction|UpdateEnemyREFfromStats))

(event Custom|setEnemyToOverWorldState
  (Class|SkeletalMeshComponent|SetAnimClass (Variables|Default|GetenemyMesh) "/Game/myModels/EnemyAnims/slimeOverworldAnimBP.slimeOverworldAnimBP_C")
  (CallFunction|UpdateEnemyREFfromStats))

(event Custom|takeTurn
  (bind _returnvalue (Game|GetGameMode))
  (bind _asbattle_game_mode (Utilities|Casting|CastTobattleGameMode _returnvalue))
  ;[1 1 1] Transferred the Take Turn Event from the old Battle Enemy BP.
  (Variables|Default|SetisEnemyTurn true)
  (Utilities|FlowControl|Delay (Variables|Default|GetenemyThinkTime))
  (if (== (Math|Random|RandomInteger 1) 0)
    (Variables|Default|SetisAttacking true)
    (else
      (Variables|Default|SetisShooting true)))
  (Variables|Default|SetisEnemyTurn false)
  (Utilities|FlowControl|Delay (Variables|/Game/BlueprintsAndMaps/Blueprints/GameBPs/battleGameMode.battleGameMode_C|GetturnDelay _asbattle_game_mode))
  (Default|EnemyFinishedTurn _asbattle_game_mode))

(event Custom|EnemySpawnProjectile
  (Development|PrintString "Slime core flies at your face!"))

(event Custom|updateEnemyREFFromStats
  (bind _enemyobject (Variables|Default|GetenemyObject))
  (bind _enemydatastructure (Variables|/Game/BlueprintsAndMaps/Blueprints/EnemyBPs/enemyObject_BP.enemyObject_BP_C|GetenemyDataStructure _enemyobject))
  (bind _enemystatsstructure (Utilities|Struct|BreakEnemyDataStructure _enemydatastructure))
  (bind (_currenthealth _maxhealth _currentlevel _basepower) (Utilities|Struct|BreakEnemyStatsStructure _enemystatsstructure))
  ;[1 1 1] SImilar concept on Player Object...but the Enemy Pawn handles its own object as I am okay with it being destroyed and re created at this point.
  (Variables|Default|SetREFCurrentHealth (Math|Conversions|ToFloat(Integer) _currenthealth))
  (Variables|Default|SetREFMaxHealth (Math|Conversions|ToFloat(Integer) _maxhealth))
  (Variables|Default|SetREFEnemyLevel _currentlevel)
  (Variables|Default|SetREFBasePower _basepower))

(event Custom|updateEnemyStatsFromREF
  ;[1 1 1] SImilar concept on Player Object...but the Enemy Pawn handles its own object as I am okay with it being destroyed and re created at this point.
  (Variables|/Game/BlueprintsAndMaps/Blueprints/EnemyBPs/enemyObject_BP.enemyObject_BP_C|SetenemyDataStructure (Variables|Default|GetenemyObject) (Utilities|Struct|MakeEnemyDataStructure (.enemyname (Variables|/Game/BlueprintsAndMaps/Blueprints/EnemyBPs/enemyObject_BP.enemyObject_BP_C|GetenemyDataStructure (Variables|Default|GetenemyObject))) (.enemyid (Variables|/Game/BlueprintsAndMaps/Blueprints/EnemyBPs/enemyObject_BP.enemyObject_BP_C|GetenemyDataStructure (Variables|Default|GetenemyObject))) (.enemymodel (Variables|/Game/BlueprintsAndMaps/Blueprints/EnemyBPs/enemyObject_BP.enemyObject_BP_C|GetenemyDataStructure (Variables|Default|GetenemyObject))) (.enemyclass (Variables|/Game/BlueprintsAndMaps/Blueprints/EnemyBPs/enemyObject_BP.enemyObject_BP_C|GetenemyDataStructure (Variables|Default|GetenemyObject))) (.enemyanimbp (Variables|/Game/BlueprintsAndMaps/Blueprints/EnemyBPs/enemyObject_BP.enemyObject_BP_C|GetenemyDataStructure (Variables|Default|GetenemyObject))) (.enemylootstructure (Variables|/Game/BlueprintsAndMaps/Blueprints/EnemyBPs/enemyObject_BP.enemyObject_BP_C|GetenemyDataStructure (Variables|Default|GetenemyObject))) (Utilities|Struct|MakeEnemyStatsStructure (Math|Float|Truncate (Variables|Default|GetREFCurrentHealth)) (Math|Float|Truncate (Variables|Default|GetREFMaxHealth)) (Variables|Default|GetREFEnemyLevel) (Variables|Default|GetREFBasePower)) (.enemyskillarray (Variables|/Game/BlueprintsAndMaps/Blueprints/EnemyBPs/enemyObject_BP.enemyObject_BP_C|GetenemyDataStructure (Variables|Default|GetenemyObject))))))

(event EventBeginPlay
  ;[1 1 1] On Begin Play Attach Face Decal Mesh to Enemy Pawn
  (Transformation|AttachComponentToComponent (Variables|Default|GetFaceMesh) (Variables|Default|GetenemyMesh) "FaceSocket" "SnapToTarget" "SnapToTarget" "SnapToTarget" true)
  (Variables|Default|SetisIdle true))

(event Collision|EventActorBeginOverlap
  (params (OtherActor :type Actor%20Object%20Reference))
  ;[1 1 1] Prevents Players from walking through Enemies. Upon something Overlapping this Enemy pawn, check to see if thats a Player Pawn and see if it is NOT Engaging, if so Stop Its movement(this may be redundant), else ignore.
  (bind _asoverworld_player_bp (Utilities|Casting|CastTooverworldPlayerBP OtherActor))
  (if (not (Variables|/Game/BlueprintsAndMaps/Blueprints/PlayerBPs/overworldPlayerBP.overworldPlayerBP_C|GetisEngaging _asoverworld_player_bp))
    (Components|Movement|StopMovementImmediately (Variables|/Script/Engine.Character|GetCharacterMovement (Game|GetPlayerCharacter 0)))))

(fn ConstructionScript)

(fn CalcDamagebySkillIndex
  (params (skillIndex :type Integer))
  (bind _enemyobject (Variables|Default|GetenemyObject))
  (bind _enemydatastructure (Variables|/Game/BlueprintsAndMaps/Blueprints/EnemyBPs/enemyObject_BP.enemyObject_BP_C|GetenemyDataStructure _enemyobject))
  (bind _enemyskillarray (Utilities|Struct|BreakEnemyDataStructure _enemydatastructure))
  (bind _output (Utilities|Array|Get(acopy) _enemyskillarray skillIndex))
  (bind _skillstatsstructure (Utilities|Struct|BreakSkillDataStructure _output))
  (bind (_mindamagepercent _maxdamagepercent) (Utilities|Struct|BreakSkillStatsStructure _skillstatsstructure))
  (return (Math|Random|RandomIntegerinRange (Math|Float|Truncate (* (Variables|Default|GetREFBasePower) _mindamagepercent)) (Math|Float|Truncate (* (Variables|Default|GetREFBasePower) _maxdamagepercent)))))

(fn SetEnemyPower
  (Variables|Default|SetREFBasePower (.basePower (Utilities|Struct|BreakEnemyStatsStructure (.enemystatsstructure (Variables|/Game/BlueprintsAndMaps/Blueprints/EnemyBPs/enemyObject_BP.enemyObject_BP_C|GetenemyDataStructure (Variables|Default|GetenemyObject)))))))