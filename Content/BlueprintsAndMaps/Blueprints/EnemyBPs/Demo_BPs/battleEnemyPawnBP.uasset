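; Demo enemy pawn for turn-based battles, carrying health in from the overworld through the game instance.
; On its turn it waits, sets an animation flag (RandomInteger(1) always picks attack over the placeholder shot), then notifies the game mode.
; Damage updates battle UI and stored health; defeat adjusts mob spawn count and destroys the actor.
; Helper functions roll skill damage from base power and data-driven percentage ranges.
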(event Custom|takeTurn
  (bind _returnvalue (Game|GetGameMode))
  (bind _asbattle_game_mode (Utilities|Casting|CastTobattleGameMode _returnvalue))
  ;[1 1 1] Event called when it is Enemy Turn on Game Mode BP.  Current prototype AI has a set 'think time' and decides whether it is Bsic Attacking or Special Attacking on a 50/50 dice roll. Sets flags for Animation which are turned off in Anim BP, and sets flag for enemy turn to disable ability to go twice.  Delay then comes from game Mode to determine how long until ENemy Finished Turn is called.
  (Variables|Default|SetisEnemyTurn true)
  (Utilities|FlowControl|Delay (Variables|Default|GetenemyThinkTime))
  (if (== (Math|Random|RandomInteger 1) 0)
    (Variables|Default|SetisAttacking true)
    (else
      (Variables|Default|SetisShooting true)))
  (Variables|Default|SetisEnemyTurn false)
  (Utilities|FlowControl|Delay (Variables|/Game/BlueprintsAndMaps/Blueprints/GameBPs/battleGameMode.battleGameMode_C|GetturnDelay _asbattle_game_mode))
  (Default|EnemyFinishedTurn _asbattle_game_mode))

(event Custom|spawnProjectile
  ;[1 1 1] Placeholder Event for Enemy Special Attack
  (Development|PrintString "Slime Shoots your face!"))

(event Custom|takeDamage
  (params (damageTaken :type Integer))
  ;[1 1 1] Enemy Takes Damage in Battle. Let the current Battle UI in Game MOde know the damage amount to display and call the Game Mode event enemy Takes Damage. CHeck to see if enemy should be defeated and if so set flag for Defeat, update Gme Instance with Enemy HP, Call Game Instance event to Upate Mob Spawn Count and delay before Destroying Actor.
  (Variables|Default|SetenemyCurrentHealth (- (Variables|Default|GetenemyCurrentHealth) (Math|Conversions|ToFloat(Integer) damageTaken)))
  (bind _asbattle_game_mode (Utilities|Casting|CastTobattleGameMode (Game|GetGameMode)))
  (Variables|/Game/BlueprintsAndMaps/Blueprints/UI_BPs/BattleUI.BattleUI_C|SetenemyDamagedNumber (Variables|/Game/BlueprintsAndMaps/Blueprints/GameBPs/battleGameMode.battleGameMode_C|GetcurrentBattleUIInstance _asbattle_game_mode) damageTaken)
  (Default|EnemyTakesDamage (Variables|/Game/BlueprintsAndMaps/Blueprints/GameBPs/battleGameMode.battleGameMode_C|GetcurrentBattleUIInstance _asbattle_game_mode) damageTaken)
  (if (<= (Variables|Default|GetenemyCurrentHealth) 0.0)
    (Variables|Default|SetisDefeated true)
    (Variables|/Game/BlueprintsAndMaps/Blueprints/GameBPs/mainGameInstance.mainGameInstance_C|SetcurrentEnemyHealth (.AsMain%20Game%20Instance (Utilities|Casting|CastTomainGameInstance (Game|GetGameInstance))) 0.0)
    (Default|ChangeMobSpawnCount (.AsMain%20Game%20Instance (Utilities|Casting|CastTomainGameInstance (Game|GetGameInstance))) 1)
    (Utilities|FlowControl|Delay 1.0)
    (Actor|DestroyActor)
    (else
      ;;[1 1 1] If Not defeated just update Current Enemy HP on Game Instance.
      (Variables|/Game/BlueprintsAndMaps/Blueprints/GameBPs/mainGameInstance.mainGameInstance_C|SetcurrentEnemyHealth (.AsMain%20Game%20Instance (Utilities|Casting|CastTomainGameInstance (Game|GetGameInstance))) (Variables|Default|GetenemyCurrentHealth)))))

(event EventBeginPlay
  ;[1 1 1] On Begin Play attach Face decal mesh to Battle Pawn and Update its HP from game instance to represent Damage dealt from possible Overworld Engage
  (Transformation|AttachComponentToComponent (Variables|Default|GetFaceMesh) (Variables|Default|GetenemyMesh) "FaceSocket" "SnapToTarget" "SnapToTarget" "KeepRelative" true)
  (Variables|Default|SetenemyCurrentHealth (Variables|/Game/BlueprintsAndMaps/Blueprints/GameBPs/mainGameInstance.mainGameInstance_C|GetcurrentEnemyHealth (.AsMain%20Game%20Instance (Utilities|Casting|CastTomainGameInstance (Game|GetGameInstance))))))

(fn ConstructionScript)

(fn CalcDamagebySkillIndex
  (params (skillIndex :type Integer))
  (bind _enemyobject (Variables|Default|Getenemyobject))
  (bind _enemydatastructure (Variables|/Game/BlueprintsAndMaps/Blueprints/EnemyBPs/enemyObject_BP.enemyObject_BP_C|GetenemyDataStructure _enemyobject))
  (bind _enemyskillarray (Utilities|Struct|BreakEnemyDataStructure _enemydatastructure))
  (bind _output (Utilities|Array|Get(acopy) _enemyskillarray skillIndex))
  (bind _skillstatsstructure (Utilities|Struct|BreakSkillDataStructure _output))
  (bind (_mindamagepercent _maxdamagepercent) (Utilities|Struct|BreakSkillStatsStructure _skillstatsstructure))
  (return (Math|Random|RandomIntegerinRange (Math|Float|Truncate (* (Variables|Default|GetREFBasePower) _mindamagepercent)) (Math|Float|Truncate (* (Variables|Default|GetREFBasePower) _maxdamagepercent)))))

(fn UpdateEnemyPower
  (Variables|Default|SetREFBasePower (.basePower (Utilities|Struct|BreakEnemyStatsStructure (.enemystatsstructure (Variables|/Game/BlueprintsAndMaps/Blueprints/EnemyBPs/enemyObject_BP.enemyObject_BP_C|GetenemyDataStructure (Variables|Default|Getenemyobject)))))))