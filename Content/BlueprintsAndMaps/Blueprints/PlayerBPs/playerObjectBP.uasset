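; Player data object that holds stats, skills and inventory, with prototype logic for power and skill damage.
; REF working variables sync both ways with PlayerStatsStructure, which can be loaded from a save game.
; It constructs skills and inventory objects from class defaults; inventory creation triggers a power calculation applying the first weapon's flat and percent passives in array order.
; Helpers find skills by type and roll damage within power-scaled ranges.
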(event Custom|updatePlayerStatsStructureFromREF
  (Variables|Default|SetplayerStatsStructure (Utilities|Struct|MakePlayerStatsStructure (Variables|Default|GetREFPlayerCurrentHealth) (Variables|Default|GetREFPlayerMaxHealth) (Variables|Default|GetREFPlayerCurrentExp) (Variables|Default|GetREFPlayerExpToNextLevel) (Variables|Default|GetREFPlayerLevel) (Variables|Default|GetREFPowerLevel) (Variables|Default|GetREFProfileName) (Variables|Default|GetREFPlayerSaveSlot) (Variables|Default|GetREFPlayerPreviousExpToNextLevel) (Variables|Default|GetREFPlayerSkillsObject) (Variables|Default|GetREFPlayerInventoryObject))))

(event Custom|updatePlayerStatsStructureFromSaveGameObject
  (params (loadedPlayerStatsStructure :type Player%20Stats%20Structure%20Structure))
  (Variables|Default|SetplayerStatsStructure loadedPlayerStatsStructure)
  (CallFunction|UpdateREFVariablesfromPlayerStatsStructure))

(event Custom|updateREFVariablesFromPlayerStatsStructure
  (bind _playerstatsstructure (Variables|Default|GetplayerStatsStructure))
  (bind _playerstatsstructure_2 (Variables|Default|GetplayerStatsStructure))
  (bind _playerstatsstructure_3 (Variables|Default|GetplayerStatsStructure))
  (bind _playerstatsstructure_4 (Variables|Default|GetplayerStatsStructure))
  (bind _playerstatsstructure_5 (Variables|Default|GetplayerStatsStructure))
  (Variables|Default|SetREFPlayerCurrentHealth (.playercurrenthealth _playerstatsstructure_2))
  (Variables|Default|SetREFPlayerMaxHealth (.playermaxhealth _playerstatsstructure_2))
  (Variables|Default|SetREFPlayerCurrentExp (.playerexp _playerstatsstructure_3))
  (Variables|Default|SetREFPlayerExpToNextLevel (.playerexptonextlevel _playerstatsstructure_3))
  (Variables|Default|SetREFPlayerPreviousExpToNextLevel (.previousplayerexptonextlevel _playerstatsstructure_4))
  (Variables|Default|SetREFPlayerLevel (.playerlevel _playerstatsstructure_4))
  (Variables|Default|SetREFProfileName (.profilename _playerstatsstructure_5))
  (Variables|Default|SetREFPlayerSaveSlot (.playersaveslot _playerstatsstructure_5))
  (Variables|Default|SetREFPlayerSkillsObject (.playerskillsobject _playerstatsstructure))
  (Variables|Default|SetREFPlayerInventoryObject (.playerinventoryobject _playerstatsstructure))
  (Variables|Default|SetREFPowerLevel (.playerbasepower _playerstatsstructure)))

(event Custom|constructInventoryObject
  ;[1 1 1] Prototype Inventory Creation. Will always pull default values from our Class Defaults of Player Inventory Object.
  (bind _returnvalue (Game|ConstructObjectfromClass "/Game/BlueprintsAndMaps/Blueprints/PlayerBPs/playerInventoryObjectBP.playerInventoryObjectBP_C" self))
  (Variables|Default|SetREFPlayerInventoryObject _returnvalue)
  (CallFunction|CalcTotalPower))

(event Custom|cosntructSkillObject
  ;[1 1 1] Prototype Skill Object Creation. Will always pull default values from our Class Defaults of Player Skills Object.
  (bind _returnvalue (Game|ConstructObjectfromClass "/Game/BlueprintsAndMaps/Blueprints/PlayerBPs/playerSkillsObjectBP.playerSkillsObjectBP_C" self))
  (Variables|Default|SetREFPlayerSkillsObject _returnvalue))

(event Custom|calcTotalPower
  (bind _refplayerinventoryobject (Variables|Default|GetREFPlayerInventoryObject))
  (bind _playerallweapons (Variables|/Game/BlueprintsAndMaps/Blueprints/PlayerBPs/playerInventoryObjectBP.playerInventoryObjectBP_C|GetplayerAllWeapons _refplayerinventoryobject))
  (bind _output (Utilities|Array|Get(acopy) _playerallweapons))
  (bind (_weapontype _weaponid _weaponname _weaponmodel _weaponpassivestructs _weaponpassivearray) (Utilities|Struct|BreakWeaponDataStructure _output))
  ;[1 1 1] Prototype to calculate total Power based off of our Weapons Passive. Only takes Power Passives from Weapon to set our Power level.
  (for (_array_element _array_index) _weaponpassivearray
    (switch Utilities|FlowControl|Switch|SwitchonWeaponPassiveTypes _array_element
      (:NewEnumerator1
        (Variables|Default|SetREFPowerLevel (+ (Variables|Default|GetREFPowerLevel) (.bonuspowerflat (Utilities|Array|Get(acopy) _weaponpassivestructs _array_index)))))
      (:NewEnumerator2
        (Variables|Default|SetREFPowerLevel (Math|Float|Truncate (* (Variables|Default|GetREFPowerLevel) (.bonuspowerpercent (Utilities|Array|Get(acopy) _weaponpassivestructs _array_index)))))))))

(fn ReturnPlayerSaveSlot
  (return (.PlayerSaveSlot (Utilities|Struct|BreakPlayerStatsStructure (Variables|Default|GetplayerStatsStructure)))))

(fn CalcDamageSkill
  (params (skillUsed :type Skill%20Data%20Structure%20Structure))
  (bind _skillstatsstructure (Utilities|Struct|BreakSkillDataStructure skillUsed))
  (bind _refpowerlevel (Variables|Default|GetREFPowerLevel))
  (bind (_mindamagepercent _maxdamagepercent) (Utilities|Struct|BreakSkillStatsStructure _skillstatsstructure))
  (return (Math|Float|Truncate (Math|Random|RandomFloatinRange (* _refpowerlevel _mindamagepercent) (* _refpowerlevel _maxdamagepercent)))))

(fn ReturnSkillbyType
  (params (skillType :type skillTypes%20Enum :default "NewEnumerator0"))
  (LocalVariables|SetdesiredSkillType skillType)
  (for _array_element (Variables|/Game/BlueprintsAndMaps/Blueprints/PlayerBPs/playerSkillsObjectBP.playerSkillsObjectBP_C|GetplayerAllSkills (Variables|Default|GetREFPlayerSkillsObject))
    (if (Utilities|Enum|Equal(Enum) (.SkillType (Utilities|Struct|BreakSkillDataStructure _array_element)) (LocalVariables|GetdesiredSkillType))
      (return _array_element))))