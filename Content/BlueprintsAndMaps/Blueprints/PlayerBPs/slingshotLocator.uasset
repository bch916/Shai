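; Slingshot aim locator actor that marks where the player is aimed and flags enemy pawns as targets.
; Each Tick before the player controller launches, it teleports to the cursor hit point mirrored through the player at a fixed height, yawing its plane relative to the player.
; Overlapping an overWorldEnemyPawnBP calls its EnemyTargeted event and shows a targeting icon material; ending overlap clears the flag and restores the grey material.
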(event Collision|EventActorBeginOverlap
  (params (OtherActor :type Actor%20Object%20Reference))
  ;[1 1 1] When this Locator actor Overlaps an Enemy Pawn it will change to a Targeting icon and let the Enemy Pawn BP know it is targeted by calling its event Enemy Targeted.
  (bind _asover_world_enemy_pawn_bp (Utilities|Casting|CastTooverWorldEnemyPawnBP OtherActor))
  (Variables|Default|SetenemyIsTargeted true)
  (Default|EnemyTargeted _asover_world_enemy_pawn_bp)
  (Rendering|Material|SetMaterial (Variables|Default|GetPlane) 0 "/Game/MyMaterials/BattleMats/Special_TripleCut_Icon_Mat.Special_TripleCut_Icon_Mat"))

(event EventTick
  (params (DeltaSeconds :type Float%20%28single-precision%29))
  (bind _returnvalue (Game|GetPlayerCharacter 0))
  (bind _returnvalue_2 (Game|GetPlayerController 0))
  (bind _returnvalue_3 (Transformation|GetActorLocation _returnvalue))
  (bind _hitresult (Game|Player|GetHitResultUnderCursorbyChannel _returnvalue_2 "TraceTypeQuery1" true))
  (bind _returnvalue_4 (* _returnvalue_3 2.0))
  (bind _location (Collision|BreakHitResult _hitresult))
  (bind _returnvalue_5 (* _location -1.0))
  (bind _returnvalue_6 (+ _returnvalue_5 _returnvalue_4))
  (bind (_x _y) (Math|Vector|BreakVector _returnvalue_6))
  ;[1 1 1] On Event Tick, check if we have NOT sent Launch command to Player pawn and if so, set the Locator position in a  reflected position across Player Pawn proportionate to Indicator Strength(for now cursor position).
  (if (not (Variables|/Game/BlueprintsAndMaps/Blueprints/PlayerBPs/playerControllerBP.playerControllerBP_C|GetlaunchedPlayer (.AsPlayer%20Controller%20BP (Utilities|Casting|CastToplayerControllerBP _returnvalue_2))))
    (Transformation|SetActorLocation (Math|Vector|MakeVector _x _y 175.0) false true)
    (Transformation|SetWorldRotation (Variables|Default|GetPlane) (Math|Rotator|MakeRotator 0.0 0.0 (- (.yaw (Math|Rotator|FindLookatRotation (Transformation|GetActorLocation) (Transformation|GetActorLocation (Game|GetPlayerCharacter 0)))) 9e+01)) false false)))

(event Collision|EventActorEndOverlap
  (params (OtherActor :type Actor%20Object%20Reference))
  ;[1 1 1] When this Locator actor Overlaps an Enemy Pawn it will change to a Targeting icon and let the Enemy Pawn BP know it is targeted by calling its event Enemy Targeted.
  (Utilities|Casting|CastTooverWorldEnemyPawnBP OtherActor)
  (Variables|Default|SetenemyIsTargeted false)
  (Rendering|Material|SetMaterial (Variables|Default|GetPlane) 0 "/Game/MyMaterials/greySGreyTarget_mat.greySGreyTarget_mat"))

(fn ConstructionScript)