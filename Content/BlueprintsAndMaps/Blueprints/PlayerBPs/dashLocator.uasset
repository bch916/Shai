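; Basic attack indicator actor that marks the player's clicked enemy target in the overworld.
; Each tick it teleports to the player controller's clicked target location at a fixed height and yaws its mesh relative to the player character.
; Overlapping an overworld enemy sets the targeted flag, notifies that enemy and shows the slash-icon material.
; Ending that overlap clears the flag and switches the mesh to a grey target material.
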(event Collision|EventActorBeginOverlap
  (params (OtherActor :type Actor%20Object%20Reference))
  ;[1 1 1] On Begin Play check if Player is already in Range and Set appropriate Material to show whether a Basic Attack engage is possible.  If Player is not In range, wait a little bit and destroy the Basic Attack Indicator and set appropriate flag on Player Controller for Basic Attack conditions.
  (bind _asover_world_enemy_pawn_bp (Utilities|Casting|CastTooverWorldEnemyPawnBP OtherActor))
  (Variables|Default|SetenemyIsTargeted true)
  (Default|EnemyTargeted _asover_world_enemy_pawn_bp)
  (Rendering|Material|SetMaterial (Variables|Default|GetbasicAttackLOcatorMesh) 0 "/Game/MyMaterials/BattleMats/Attack_Slash_Icon_Mat.Attack_Slash_Icon_Mat"))

(event EventTick
  (params (DeltaSeconds :type Float%20%28single-precision%29))
  ;[1 1 1] On Event tick keep rotating the Basic Attack Locator at the Player postion and checking if still in range. This whole functionality and class should be put on the Enemy and use the engines Basic Attack event that is built-in.
  (bind _asplayer_controller_bp (Utilities|Casting|CastToplayerControllerBP (Game|GetPlayerController 0)))
  (Transformation|SetActorLocation (Math|Vector|MakeVector (.x (Variables|/Game/BlueprintsAndMaps/Blueprints/PlayerBPs/playerControllerBP.playerControllerBP_C|GettargetedEnemyLocationOnClick _asplayer_controller_bp)) (.y (Variables|/Game/BlueprintsAndMaps/Blueprints/PlayerBPs/playerControllerBP.playerControllerBP_C|GettargetedEnemyLocationOnClick _asplayer_controller_bp)) 1.6e+02) false true)
  (Transformation|SetWorldRotation (Variables|Default|GetbasicAttackLOcatorMesh) (Math|Rotator|MakeRotator 0.0 0.0 (- (.yaw (Math|Rotator|FindLookatRotation (Transformation|GetActorLocation) (Transformation|GetActorLocation (Game|GetPlayerCharacter 0)))) 9e+01)) false false))

(event Collision|EventActorEndOverlap
  (params (OtherActor :type Actor%20Object%20Reference))
  ;[1 1 1] On Begin Play check if Player is already in Range and Set appropriate Material to show whether a Basic Attack engage is possible.  If Player is not In range, wait a little bit and destroy the Basic Attack Indicator and set appropriate flag on Player Controller for Basic Attack conditions.
  (Utilities|Casting|CastTooverWorldEnemyPawnBP OtherActor)
  (Variables|Default|SetenemyIsTargeted false)
  (Rendering|Material|SetMaterial (Variables|Default|GetbasicAttackLOcatorMesh) 0 "/Game/MyMaterials/greySGreyTarget_mat.greySGreyTarget_mat"))

(fn ConstructionScript)