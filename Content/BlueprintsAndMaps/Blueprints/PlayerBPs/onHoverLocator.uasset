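; Hover indicator actor showing whether the player can engage a basic attack on the hovered enemy.
; Each tick it moves to the player controller's hovered-enemy position at a fixed height and yaws toward the player.
; It swaps between in-range and out-of-range slash icons based on max dash distance.
; When out of range, it waits briefly, clears the locator flags on controller and enemy, then destroys itself.
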(event EventTick
  (params (DeltaSeconds :type Float%20%28single-precision%29))
  ;[1 1 1] On Event tick keep rotating the Hover Locator at the Player postion and checking if still in range. This whole functionality and class should be put on the Enemy and use the engines On Hover event that is built-in.
  (bind _asplayer_controller_bp (Utilities|Casting|CastToplayerControllerBP (Game|GetPlayerController 0)))
  (Transformation|SetActorLocation (Math|Vector|MakeVector (.x (Variables|/Game/BlueprintsAndMaps/Blueprints/PlayerBPs/playerControllerBP.playerControllerBP_C|GettargetedEnemyMouseHover _asplayer_controller_bp)) (.y (Variables|/Game/BlueprintsAndMaps/Blueprints/PlayerBPs/playerControllerBP.playerControllerBP_C|GettargetedEnemyMouseHover _asplayer_controller_bp)) 175.0) false true)
  (Transformation|SetWorldRotation (Variables|Default|GetHoverLocatorMesh) (Math|Rotator|MakeRotator 0.0 0.0 (- (.yaw (Math|Rotator|FindLookatRotation (Transformation|GetActorLocation) (Transformation|GetActorLocation (Game|GetPlayerCharacter 0)))) 9e+01)) false false)
  (bind _asplayer_controller_bp_2 (Utilities|Casting|CastToplayerControllerBP (Game|GetPlayerController 0)))
  (if (< (Math|Vector|VectorLength (- (Variables|/Game/BlueprintsAndMaps/Blueprints/PlayerBPs/playerControllerBP.playerControllerBP_C|GettargetedEnemyMouseHover _asplayer_controller_bp_2) (Transformation|GetActorLocation (Game|GetPlayerCharacter 0)))) (Variables|/Game/BlueprintsAndMaps/Blueprints/PlayerBPs/playerControllerBP.playerControllerBP_C|GetmaxDashDistance _asplayer_controller_bp_2))
    (Rendering|Material|SetMaterial (Variables|Default|GetHoverLocatorMesh) 0 "/Game/MyMaterials/onHover_Attack_Slash_Icon_Mat.onHover_Attack_Slash_Icon_Mat")
    (else
      (Rendering|Material|SetMaterial (Variables|Default|GetHoverLocatorMesh) 0 "/Game/MyMaterials/onHover_Attack_Slash_OutOfRange_Icon_Mat.onHover_Attack_Slash_OutOfRange_Icon_Mat")
      (Utilities|FlowControl|Delay 0.25)
      (Variables|/Game/BlueprintsAndMaps/Blueprints/PlayerBPs/playerControllerBP.playerControllerBP_C|SethasSpawnedOnHoverLocator (.AsPlayer%20Controller%20BP (Utilities|Casting|CastToplayerControllerBP (Game|GetPlayerController 0))) false)
      (Variables|/Game/BlueprintsAndMaps/Blueprints/EnemyBPs/overWorldEnemyPawnBP.overWorldEnemyPawnBP_C|SethasALocator (Variables|Default|GettargetedEnemy) false)
      (Actor|DestroyActor))))

(event EventBeginPlay
  ;[1 1 1] On Begin Play check if Player is already in Range and Set appropriate Material to show whether a Basic Attack engage is possible.  If Player is not In range, wait a little bit and destroy the Hover Indicator and set appropriate flag on Player Controller for Basic Attack conditions.
  (if (Variables|Default|GetplayerInRange)
    (Rendering|Material|SetMaterial (Variables|Default|GetHoverLocatorMesh) 0 "/Game/MyMaterials/onHover_Attack_Slash_Icon_Mat.onHover_Attack_Slash_Icon_Mat")
    (else
      (Rendering|Material|SetMaterial (Variables|Default|GetHoverLocatorMesh) 0 "/Game/MyMaterials/onHover_Attack_Slash_OutOfRange_Icon_Mat.onHover_Attack_Slash_OutOfRange_Icon_Mat")
      (Utilities|FlowControl|Delay 0.25)
      (Variables|/Game/BlueprintsAndMaps/Blueprints/PlayerBPs/playerControllerBP.playerControllerBP_C|SethasSpawnedOnHoverLocator (.AsPlayer%20Controller%20BP (Utilities|Casting|CastToplayerControllerBP (Game|GetPlayerController 0))) false)
      (Variables|/Game/BlueprintsAndMaps/Blueprints/EnemyBPs/overWorldEnemyPawnBP.overWorldEnemyPawnBP_C|SethasALocator (Variables|Default|GettargetedEnemy) false)
      (Actor|DestroyActor))))

(fn ConstructionScript)