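; Overworld camera actor that follows the player and hides rigidBodyActor objects that get in the way.
; On BeginPlay it takes its saved position from the main game instance, intended to restore the spot after battle.
; Each Tick it holds a fixed height and offset behind the player along X, sweeping a sphere to a point ahead of the camera.
; Overlaps with that sphere toggle those actors' visibility off and back on.
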(event EventBeginPlay
  ;[1 1 1] On Camera begin play get Position from Game Instance to handle putting in same spot after Battle.
  (bind _asmain_game_instance (Utilities|Casting|CastTomainGameInstance (Game|GetGameInstance)))
  (Transformation|SetActorLocation (Variables|/Game/BlueprintsAndMaps/Blueprints/GameBPs/mainGameInstance.mainGameInstance_C|GetoverworldCameraPosition _asmain_game_instance) false false))

(event EventTick
  (params (DeltaSeconds :type Float%20%28single-precision%29))
  (bind _returnvalue (Game|GetPlayerCharacter 0))
  (bind _returnvalue_2 (Transformation|GetActorLocation _returnvalue))
  (bind (_x _y) (Math|Vector|BreakVector _returnvalue_2))
  ;[1 1 1] On event tick, keep the Camera and Sphere Locator at the correct positions at all times. There may be a better way to do this.
  (Transformation|SetActorLocation (Math|Vector|MakeVector (- _x 7e+02) _y 1e+03) false false)
  (Transformation|SetWorldLocation (Variables|Default|GetSphere) (+ (Transformation|GetWorldLocation (Variables|Default|GetCamera)) (* (Math|Vector|GetForwardVector (Transformation|GetWorldRotation (Variables|Default|GetCamera))) 7.5e+02)) true false))

(event Collision|EventActorBeginOverlap
  (params (OtherActor :type Actor%20Object%20Reference))
  ;[1 1 1] Using the Overworld Cameras Sphere Collider, we can toggle the Visibility of Rigid Body Actors in the world on Begin and End Overlap respectively.
  (if (Collision|IsOverlappingActor (Variables|Default|GetSphere) OtherActor :!class /Script/Engine.PrimitiveComponent)
    (bind _asrigid_body_actor (Utilities|Casting|CastTorigidBodyActor OtherActor))
    (Default|ToggleVisibility _asrigid_body_actor false)))

(event Collision|EventActorEndOverlap
  (params (OtherActor :type Actor%20Object%20Reference))
  ;[1 1 1] Using the Overworld Cameras Sphere Collider, we can toggle the Visibility of Rigid Body Actors in the world on Begin and End Overlap respectively.
  (if (not (Collision|IsOverlappingActor (Variables|Default|GetSphere) OtherActor :!class /Script/Engine.PrimitiveComponent))
    (bind _asrigid_body_actor (Utilities|Casting|CastTorigidBodyActor OtherActor))
    (Default|ToggleVisibility _asrigid_body_actor true)))

(fn ConstructionScript)