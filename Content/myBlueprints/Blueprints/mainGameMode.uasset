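; Game mode for the overworld that adds the overworld UI on BeginPlay and handles enemy spawning and battle transitions.
; Spawning places an enemy pawn at a random point and yaw around the current spawn origin and radius, then updates the mob count in the game instance.
; Going to battle shows a start screen, saves camera and player locations to the game instance, then opens BattleMap after a delay.
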(event Custom|spawnNewEnemy
  (bind _currentspawnorigin (Variables|Default|GetcurrentSpawnOrigin))
  (bind _currentspawnradius (Variables|Default|GetcurrentSpawnRadius))
  (bind _currentspawnradius_2 (Variables|Default|GetcurrentSpawnRadius))
  ;[1 1 1] Game Mode can Spawn new Enemies and takes a Spawn Origin point(middle of tile) and from a given Spawn Radius, picks a random point and random rotation to Spawn in Overworld.
  (bind _output_get (Variables|Default|SetspawnOffset (Math|Vector|MakeVector (+ (Math|Random|RandomFloatinRange (* _currentspawnradius_2 -1.0) _currentspawnradius_2) (.x _currentspawnorigin)) (+ (Math|Random|RandomFloatinRange (* -1.0 _currentspawnradius) _currentspawnradius) (.y _currentspawnorigin)) (.z _currentspawnorigin))))
  (Variables|Default|SetspawnTransform (Math|Transform|MakeTransform _output_get (Math|Rotator|MakeRotator 0.0 0.0 (Math|Random|RandomFloatinRange 1.3e+02 2.3e+02))))
  (Game|SpawnActorfromClass "/Game/myBlueprints/Blueprints/overWorldEnemyPawnBP.overWorldEnemyPawnBP_C" (Variables|Default|GetspawnTransform) "AdjustIfPossibleButDontSpawnIfColliding" 0 0 0)
  (Default|ChangeMobSpawnCount (.AsMain%20Game%20Instance (Utilities|Casting|CastTomainGameInstance (Game|GetGameInstance))) 1))

(event Custom|sendToBattle
  ;[1 1 1] Game Mode sends Player To BattleMap and stores the Camera and Players positions to spawn them there after Battle.
  (bind _returnvalue (UserInterface|CreateWidget "/Game/myBlueprints/Blueprints/HUD/battleStartScreen.battleStartScreen_C" (Game|GetPlayerController 0)))
  (UserInterface|Viewport|AddtoViewport _returnvalue 0)
  (bind _outactors (Actor|GetAllActorsOfClass "/Game/myBlueprints/Blueprints/OverworldCameaBP.OverworldCameaBP_C"))
  (Variables|/Game/myBlueprints/Blueprints/mainGameInstance.mainGameInstance_C|SetoverworldCameraOrigin (.AsMain%20Game%20Instance (Utilities|Casting|CastTomainGameInstance (Game|GetGameInstance))) (Transformation|GetActorLocation (Utilities|Array|Get(acopy) _outactors)))
  (Variables|/Game/myBlueprints/Blueprints/mainGameInstance.mainGameInstance_C|SetoverworldPlayerOrigin (.AsMain%20Game%20Instance (Utilities|Casting|CastTomainGameInstance (Game|GetGameInstance))) (Transformation|GetActorLocation (Game|GetPlayerCharacter 0)))
  (Utilities|FlowControl|Delay (Variables|Default|GetOverworldToBattleMapDelay))
  (Game|OpenLevel(byName) "BattleMap"))

(event EventBeginPlay
  ;[1 1 1] On Game Mode Begin Play, Add Overworld UI, set it locally and Add it to viewport.
  (bind _returnvalue (UserInterface|CreateWidget "/Game/myBlueprints/Blueprints/HUD/OverworldUI.OverworldUI_C" (Game|GetPlayerController 0)))
  (bind _output_get (Variables|Default|SetcurrentOverworldUI _returnvalue))
  (UserInterface|Viewport|AddtoViewport _output_get 0))

(fn ConstructionScript)