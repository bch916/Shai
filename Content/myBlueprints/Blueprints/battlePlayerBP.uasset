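; Player pawn Blueprint for turn-based battles, handling health, damage, recharge healing and turn end.
; On BeginPlay it attaches a face mesh to a socket and loads health from mainGameInstance.
; Damage updates the battle UI and Game Instance, with a random roll on lethal hits to survive at 1 HP.
; Recharge heals the stored health up to max and reloads it; turn end notifies battleGameMode after a delay.
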(event Custom|endTurn
  ;[1 1 1] Event to End Player Turn on Game Mode BP
  (Utilities|FlowControl|Delay (Variables|/Game/myBlueprints/Blueprints/battleGameMode.battleGameMode_C|GetturnDelay (.AsBattle%20Game%20Mode (Utilities|Casting|CastTobattleGameMode (Game|GetGameMode)))))
  (Default|PlayerFinishedTurn (.AsBattle%20Game%20Mode (Utilities|Casting|CastTobattleGameMode (Game|GetGameMode)))))

(event Custom|takeDamage
  (params (damageTaken :type Integer))
  ;[1 1 1] Player Takes Damage. Subtract incoming damage from Players current HP
  (Variables|Default|SetplayerCurrentHealth (- (Variables|Default|GetplayerCurrentHealth) (Math|Conversions|ToFloat(Integer) damageTaken)))
  ;[1 1 1] To display the Damage dealt we let the Game Modes current Battle UI know the Damage amount.
  (bind _asbattle_game_mode (Utilities|Casting|CastTobattleGameMode (Game|GetGameMode)))
  (Default|PlayerTakesDamage (Variables|/Game/myBlueprints/Blueprints/battleGameMode.battleGameMode_C|GetcurrentBattleUIInstance _asbattle_game_mode) damageTaken)
  ;[1 1 1] Check if Player should be defeated.
  (if (<= (Variables|Default|GetplayerCurrentHealth) 0.0)
    ;[1 1 1] Second Chance to live is rolled here. Then Update Player on Game Instance with Player Defeated flag.
    (switch int (Math|Random|RandomInteger 2)
      (:0
        (CallFunction|UpdatePlayeronGameInstance true))
      (:1
        (Variables|Default|SetplayerCurrentHealth 1.0 :!label _label)
        (CallFunction|UpdatePlayeronGameInstance false))
      (:2
        (goto _label)))
    (else
      ;[1 1 1] Updates Player Health from this blueprint to Game Instance.
      (CallFunction|UpdatePlayeronGameInstance false))))

(event Custom|updatePlayerOnGameInstance
  (params (wasPlayerDefeated :type Boolean))
  ;[1 1 1] Update Player Statuses on Game Instance.
  (bind _asmain_game_instance (Utilities|Casting|CastTomainGameInstance (Game|GetGameInstance)))
  (Variables|/Game/myBlueprints/Blueprints/mainGameInstance.mainGameInstance_C|SetREF_playerCurrentHealth _asmain_game_instance (Variables|Default|GetplayerCurrentHealth))
  (Variables|/Game/myBlueprints/Blueprints/mainGameInstance.mainGameInstance_C|SetREF_playerMaxHealth _asmain_game_instance (Variables|Default|GetplayerMaxHealth))
  (Variables|/Game/myBlueprints/Blueprints/mainGameInstance.mainGameInstance_C|SetplayerDefeated _asmain_game_instance wasPlayerDefeated))

(event Custom|updatePlayerFromGameInstance
  ;[1 1 1] Event is used to Update Player here locally from Game Instance. Usually on Begin Play or after a Battle.
  (bind _asmain_game_instance (Utilities|Casting|CastTomainGameInstance (Game|GetGameInstance)))
  (Variables|Default|SetplayerCurrentHealth (Variables|/Game/myBlueprints/Blueprints/mainGameInstance.mainGameInstance_C|GetREF_playerCurrentHealth _asmain_game_instance))
  (Variables|Default|SetplayerMaxHealth (Variables|/Game/myBlueprints/Blueprints/mainGameInstance.mainGameInstance_C|GetREF_playerMaxHealth _asmain_game_instance)))

(event Custom|updatePlayerHealthFromRecharge
  (params (changedHealth :type Integer))
  ;[1 1 1] Event called to Update Players Health for Recharge Ability.  This could possibly be merged with Take Damage in such a way that we could add or subtract HP there and know the condition and dam,age dealr/healing source.
  (bind _asmain_game_instance (Utilities|Casting|CastTomainGameInstance (Game|GetGameInstance)))
  (if (>= (+ (Math|Conversions|ToFloat(Integer) changedHealth) (Variables|/Game/myBlueprints/Blueprints/mainGameInstance.mainGameInstance_C|GetREF_playerCurrentHealth (.AsMain%20Game%20Instance (Utilities|Casting|CastTomainGameInstance (Game|GetGameInstance))))) (Variables|/Game/myBlueprints/Blueprints/mainGameInstance.mainGameInstance_C|GetREF_playerMaxHealth _asmain_game_instance))
    (Variables|/Game/myBlueprints/Blueprints/mainGameInstance.mainGameInstance_C|SetREF_playerCurrentHealth (.AsMain%20Game%20Instance (Utilities|Casting|CastTomainGameInstance (Game|GetGameInstance))) (Variables|/Game/myBlueprints/Blueprints/mainGameInstance.mainGameInstance_C|GetREF_playerMaxHealth _asmain_game_instance))
    (else
      (Variables|/Game/myBlueprints/Blueprints/mainGameInstance.mainGameInstance_C|SetREF_playerCurrentHealth (.AsMain%20Game%20Instance (Utilities|Casting|CastTomainGameInstance (Game|GetGameInstance))) (+ (Math|Conversions|ToFloat(Integer) changedHealth) (Variables|/Game/myBlueprints/Blueprints/mainGameInstance.mainGameInstance_C|GetREF_playerCurrentHealth (.AsMain%20Game%20Instance (Utilities|Casting|CastTomainGameInstance (Game|GetGameInstance))))))))
  (CallFunction|UpdatePlayerfromGameInstance))

(event EventBeginPlay
  ;[1 1 1] At Begin Play attach face decal mesh to Player Pawn. Then update the Player from the Game Instance with Statuses
  (Transformation|AttachComponentToComponent (Variables|Default|GetFaceMesh) (Variables|Character|GetMesh) "FaceSocket" "SnapToTarget" "SnapToTarget" "SnapToTarget" true)
  (CallFunction|UpdatePlayerfromGameInstance))

(fn ConstructionScript)