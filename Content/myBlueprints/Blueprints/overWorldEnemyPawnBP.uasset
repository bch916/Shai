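; Overworld enemy pawn that players can target and damage until it is defeated.
; It snaps a face mesh to the body's socket, tracks idle and reacting states, and halts a non-engaging player who overlaps it.
; Damage lowers health and shows on the game mode's overworld UI.
; Surviving health is saved to the game instance, while defeat updates its mob spawn count and destroys the pawn after a delay.
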(event Custom|enemyTargeted
  ;[1 1 1] Interaction from Player Controller can call this event to set Enemy into Reacting State
  (Variables|Default|SetisReacting true))

(event Custom|takeDamage
  (params (damageNumber :type Integer))
  ;[1 1 1] Enemy Takes Damage.  Subtract incoming damage from health and pass the damage number to the Game Modes Current UI to display dmg.
  (Variables|Default|SetenemyCurrentHealth (- (Variables|Default|GetenemyCurrentHealth) (Math|Conversions|ToFloat(Integer) damageNumber)))
  (bind _asmain_game_mode (Utilities|Casting|CastTomainGameMode (Game|GetGameMode)))
  (Variables|/Game/myBlueprints/Blueprints/HUD/OverworldUI.OverworldUI_C|SetenemyDamagedNumber (Variables|/Game/myBlueprints/Blueprints/mainGameMode.mainGameMode_C|GetcurrentOverworldUI _asmain_game_mode) damageNumber)
  (Default|EnemyTakesDamage (Variables|/Game/myBlueprints/Blueprints/mainGameMode.mainGameMode_C|GetcurrentOverworldUI _asmain_game_mode) damageNumber)
  ;[1 1 1] Check if Damage is defating the Enemy and if so set Flag fo Defeated and call Change Mob Spawn Count on Game Instance. Delay 1 second and DEstroy the Enemy Pawn.
  (if (<= (Variables|Default|GetenemyCurrentHealth) 0.0)
    (Variables|Default|SetisDefeated true)
    (Default|ChangeMobSpawnCount (.AsMain%20Game%20Instance (Utilities|Casting|CastTomainGameInstance (Game|GetGameInstance))) 1)
    (Utilities|FlowControl|Delay 1.0)
    (Actor|DestroyActor)
    (else
      (Variables|/Game/myBlueprints/Blueprints/mainGameInstance.mainGameInstance_C|SetcurrentEnemyHealth (.AsMain%20Game%20Instance (Utilities|Casting|CastTomainGameInstance (Game|GetGameInstance))) (Variables|Default|GetenemyCurrentHealth)))))

(event EventBeginPlay
  ;[1 1 1] On Begin Play Attach Face Decal Mesh to Enemy Pawn
  (Transformation|AttachComponentToComponent (Variables|Default|GetFaceMesh) (Variables|Default|GetenemyMesh) "FaceSocket" "SnapToTarget" "SnapToTarget" "SnapToTarget" true)
  (Variables|Default|SetisIdle true))

(event Collision|EventActorBeginOverlap
  (params (OtherActor :type Actor%20Object%20Reference))
  ;[1 1 1] Prevents Players from walking through Enemies. Upon something Overlapping this Enemy pawn, check to see if thats a Player Pawn and see if it is NOT Engaging, if so Stop Its movement(this may be redundant), else ignore.
  (bind _asoverworld_player_bp (Utilities|Casting|CastTooverworldPlayerBP OtherActor))
  (if (not (Variables|/Game/myBlueprints/Blueprints/overworldPlayerBP.overworldPlayerBP_C|GetisEngaging _asoverworld_player_bp))
    (Components|Movement|StopMovementImmediately (Variables|/Script/Engine.Character|GetCharacterMovement (Game|GetPlayerCharacter 0)))))

(fn ConstructionScript)