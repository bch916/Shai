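; Slingshot pull indicator actor that visualises the rubber-band stretch between the mouse cursor and the player character.
; Each tick it moves to the cursor's hit point at a fixed height and rotates its Cube to face the player.
; Its X scale follows the flattened cursor-to-player distance divided by a modifier, showing pull strength.
; It destroys itself once the player controller reports a launch or the mouse is released.
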(event EventTick
  (params (DeltaSeconds :type Float%20%28single-precision%29))
  (bind _returnvalue (Game|GetPlayerCharacter 0))
  (bind _returnvalue_2 (Game|GetPlayerController 0))
  (bind _indicatordefaultyzscale (Variables|Default|GetIndicatorDefaultYZScale))
  (bind _hitresult (Game|Player|GetHitResultUnderCursorbyChannel _returnvalue_2 "TraceTypeQuery1" true))
  (bind _returnvalue_3 (Transformation|GetActorLocation _returnvalue))
  (bind (_x _y) (Math|Vector|BreakVector (.location _hitresult)))
  ;[1 1 1] On Event Tick set the Indicator at cursor postion, rotate it towards actor and scale it with a modifier to indicate the strength of the pull. This is the rubber band effect of slingshotting so far.
  (Transformation|SetActorLocation (Math|Vector|MakeVector _x _y 1.6e+02) false true)
  (Variables|Default|SetInidcatorCurrentXScale (/ (Math|Vector|VectorLength (- (Math|Vector|MakeVector _x _y 0.0) (Math|Vector|MakeVector (.x _returnvalue_3) (.y _returnvalue_3) 0.0))) (Variables|Default|GetindicatorScaleModifier)))
  (Transformation|SetWorldRotation (Variables|Default|GetCube) (Math|Rotator|FindLookatRotation (Transformation|GetActorLocation) (Transformation|GetActorLocation (Game|GetPlayerCharacter 0))) false false)
  (Transformation|SetActorScale3D (Math|Vector|MakeVector (Variables|Default|GetInidcatorCurrentXScale) _indicatordefaultyzscale _indicatordefaultyzscale))
  (if (or (Variables|/Game/myBlueprints/Blueprints/playerControllerBP.playerControllerBP_C|GetlaunchedPlayer (.AsPlayer%20Controller%20BP (Utilities|Casting|CastToplayerControllerBP (Game|GetPlayerController 0)))) (Variables|Default|GetmouseReleased))
    (Actor|DestroyActor)))

(fn ConstructionScript)